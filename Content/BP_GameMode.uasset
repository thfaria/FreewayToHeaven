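; Game mode for a one- or two-player chicken road-crossing level, with count-up or Time Trial timer set from the Game Instance.
; Buses feed chickens one at a time to each player's controller; saves and road kills update scores and HUD, then possess the next.
; Resistance and speed power-ups modify chickens, with surviving hits hopping forward.
; Empty buses or expired time switch to the end camera, results screen and spawned tombstones.
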(event EventBeginPlay
  ;[0.15 0.15 0.15 0.5] Inicia a fase - busca a quantidade de jogadores selecionados no menu e o modo de jogo (armazenados no Game Instance)
  (bind _asbp_my_game_instance (Utilities|Casting|CastToBP_MyGameInstance (Game|GetGameInstance)))
  (Variables|Default|SetTimeTrial (Variables|/Game/BP_MyGameInstance.BP_MyGameInstance_C|GetTimeTrial? _asbp_my_game_instance))
  (bind _output_get (Variables|Default|Set2Players (Variables|/Game/BP_MyGameInstance.BP_MyGameInstance_C|Get2Players? _asbp_my_game_instance)))
  (if _output_get
    (Class|GameplayStatics|CreatePlayer 1))
  (CallFunction|IniciaFase))

(event EventTick
  (params (DeltaSeconds :type Float%20%28single-precision%29))
  ;[0.15 0.15 0.15 0.5] Atualiza o tempo do jogo de acordo com o modo escolhido no menu. Se for Time Trial verifica se o tempo zerou e chama o final da fase
  (if (Variables|Default|GetLevelGo)
    (if (Variables|Default|GetTimeTrial)
      (bind _output_get (Variables|Default|SetTimer (- (Variables|Default|GetTimer) DeltaSeconds)))
      (if (<= _output_get 0.0)
        (CallFunction|FimFase)
        (else
          (CallFunction|UpdateHUDTempo :!label _label)))
      (else
        (Variables|Default|SetTimer (+ (Variables|Default|GetTimer) DeltaSeconds))
        (goto _label)))))

(fn ConstructionScript)

(fn GalinhaSalva
  (params (GalinhaRef :type BP%20Galinha%20Object%20Reference))
  ;[0.15 0.15 0.15 0.5] Função que contabiliza a entrega da Galinha na igreja
  (if (Variables|/Game/BP_Galinha.BP_Galinha_C|GetPlayer2? GalinhaRef)
    (bind _result (Math|Integer|IncrementInt (Variables|Default|GetGalinhasSalvas_P2))
      (:%20%20
        (Variables|Default|SetGalinhasSalvas_P2 _result)
        (Variables|Default|SetProxGalinha 2)))
    (else
      (bind _result_2 (Math|Integer|IncrementInt (Variables|Default|GetGalinhasSalvas_P1))
        (:%20%20
          (Variables|Default|SetGalinhasSalvas_P1 _result_2)
          (Variables|Default|SetProxGalinha 1)))))
  (CallFunction|UpdateHUDGalinhasSalvas)
  (Actor|DestroyActor GalinhaRef)
  (CallFunction|ProximaGalinha))

(fn GalinhaAtropelada
  (params (GalinhaRef :type BP%20Galinha%20Object%20Reference))
  (bind _returnvalue (Transformation|GetActorLocation GalinhaRef))
  ;[0.15 0.15 0.15 0.5] Diminui a vida da Galinha e, caso seja zerada, contabiliza o atropelamento.
  (bind _result (Math|Integer|DecrementInt (Variables|/Game/BP_Galinha.BP_Galinha_C|GetResistencia GalinhaRef))
    (:%20%20
      (bind _output_get (Variables|/Game/BP_Galinha.BP_Galinha_C|SetResistencia GalinhaRef _result))
      (if (== _output_get 0)
        (Game|SpawnActorfromClass "/Game/BP_Atropelamento.BP_Atropelamento_C" (Math|Transform|MakeTransform (Math|Vector|MakeVector (.x _returnvalue) (.y _returnvalue) 0.0) "0, 0, 0" "1.000000,1.000000,1.000000") "Undefined" "MultiplyWithRoot" 0 0)
        (Game|SpawnActorfromClass "/Game/BP_Alma.BP_Alma_C" (Math|Transform|MakeTransform (Math|Vector|MakeVector (.x _returnvalue) (.y _returnvalue) 3e+01) "0, 0, 0" "1.000000,1.000000,1.000000") "Undefined" "MultiplyWithRoot" 0 0)
        (if (Variables|/Game/BP_Galinha.BP_Galinha_C|GetPlayer2? GalinhaRef)
          (bind _result_2 (Math|Integer|IncrementInt (Variables|Default|GetGalinhasAtropeladas_P2))
            (:%20%20
              (Variables|Default|SetGalinhasAtropeladas_P2 _result_2)
              (Variables|Default|SetProxGalinha 2)))
          (else
            (bind _result_3 (Math|Integer|IncrementInt (Variables|Default|GetGalinhasAtropeladas_P1))
              (:%20%20
                (Variables|Default|SetGalinhasAtropeladas_P1 _result_3)
                (Variables|Default|SetProxGalinha 1)))))
        (CallFunction|UpdateHUDGalinhasAtropeladas)
        (Actor|DestroyActor GalinhaRef)
        (CallFunction|ProximaGalinha)
        (else
          (CallFunction|PuloGalinha GalinhaRef))))))

(fn ProximaGalinha
  (bind _proxgalinha (Variables|Default|GetProxGalinha))
  ;[0.15 0.15 0.15 0.5] Função que chama a próxima galinha do ônibus de acordo com a Variável ProxGalinha (1-Carrega P1, 2-Carrega P2, 0-Carrega ambas). Atualiza a quantidade no ônibus, verifica o final de jogo e, se não tiver terminado, carrega a galinha e dá o controle ao jogador.
  (if (== _proxgalinha 1)
    ;;[0.15 0.15 0.15 0.5] Galinha Player 1
    (CallFunction|AtualizaOnibus true)
    (if (< (Variables|Default|GetGalinhasOnibus_P1) 0)
      (CallFunction|VerificaFimFase)
      (else
        (CallFunction|UpdateHUDGalinhasOnibus)
        (CallFunction|CarregaGalinha true)))
    (else
      ;;[0.15 0.15 0.15 0.5] Galinha Player 2
      (if (== _proxgalinha 2)
        (CallFunction|AtualizaOnibus false)
        (if (< (Variables|Default|GetGalinhasOnibus_P2) 0)
          (CallFunction|VerificaFimFase)
          (else
            (CallFunction|UpdateHUDGalinhasOnibus)
            (CallFunction|CarregaGalinha false)))
        (else
          ;;[0.15 0.15 0.15 0.5] Ambas
          (CallFunction|AtualizaOnibus true)
          (CallFunction|AtualizaOnibus false)
          (CallFunction|UpdateHUDGalinhasOnibus)
          (CallFunction|CarregaGalinha true)
          (CallFunction|CarregaGalinha false))))))

(fn PowerUpColetado
  (params (GalinhaRef :type BP%20Galinha%20Object%20Reference) (PowerUp_Tipo :type Integer))
  ;[0.15 0.15 0.15 0.5] Função do PowerUp coletado pelo jogador. Dependendo do tipo chama o efeito
  (if (== PowerUp_Tipo 1)
    (CallFunction|PowerUpEfeitoVelocidade GalinhaRef)
    (else
      (CallFunction|PowerUpEfeitoResistencia GalinhaRef))))

(fn FimFase
  ;[0.15 0.15 0.15 0.5] Muda para a Camera de Final de Fase, chama a tela de Final da Fase e atualiza os valores do jogo na mesma
  (Variables|Default|SetLevelGo false)
  (CallFunction|ResetElementos "/Game/BP_Galinha.BP_Galinha_C")
  (CallFunction|RemoveHud)
  (bind _outactors (Actor|GetAllActorsOfClasswithTag "/Script/CinematicCamera.CineCameraActor" "CameraFinalFase"))
  (Game|Player|SetViewTargetwithBlend (Game|GetPlayerController 0) (Utilities|Array|Get(acopy) _outactors) 2.0 "VTBlend_EaseInOut" 2.0 false)
  (if (< (Variables|Default|GetTimer) 0.0)
    (Variables|Default|SetTimer 0.0))
  (bind _returnvalue (UserInterface|CreateWidget "/Game/_Widgets/WBP_EndLevel.WBP_EndLevel_C"))
  (bind _output_get (Variables|Default|SetTelaFinal _returnvalue))
  (UserInterface|Viewport|AddtoViewport _output_get 0)
  (Default|UpdateEndLevelScreen _output_get (Variables|Default|GetGalinhasAtropeladas_P1) (Variables|Default|GetGalinhasSalvas_P1) (Variables|Default|GetGalinhasAtropeladas_P2) (Variables|Default|GetGalinhasSalvas_P2) (Variables|Default|GetTimer))
  (CallFunction|CarregaLapides)
  (CallFunction|SetControleMouse))

(fn RemoveTelaFinal
  (bind _telafinal (Variables|Default|GetTelaFinal))
  ;[0.15 0.15 0.15 0.5] Verifica se a tela de final de fase existe e então remove a mesma
  (Utilities|IsValid _telafinal
    (:Is%20Valid
      (Widget|RemovefromParent _telafinal))))

(fn IniciaFase
  ;[0.15 0.15 0.15 0.5] Sequencia de ações para o reinício da fase
  (CallFunction|SetControleTeclado)
  (CallFunction|RemoveTelaFinal)
  (CallFunction|ResetaVariaveis)
  (CallFunction|CarregaHUD)
  (CallFunction|UpdateHUDGalinhasAtropeladas)
  (CallFunction|UpdateHUDGalinhasSalvas)
  (CallFunction|UpdateHUDTempo)
  (CallFunction|UpdateHUDGalinhasOnibus)
  (CallFunction|ResetSpawns)
  (CallFunction|ResetElementos "/Game/BP_Galinha.BP_Galinha_C")
  (CallFunction|ResetElementos "/Game/BP_Veiculo.BP_Veiculo_C")
  (CallFunction|ResetElementos "/Game/BP_PowerUp.BP_PowerUp_C")
  (CallFunction|ResetElementos "/Game/BP_Atropelamento.BP_Atropelamento_C")
  (CallFunction|ResetElementos "/Game/BP_Alma.BP_Alma_C")
  (CallFunction|ResetElementos "/Game/BP_Lapide.BP_Lapide_C")
  (CallFunction|CarregaOnibusP2)
  (CallFunction|ProximaGalinha))

(fn ResetaVariaveis
  (bind _galinhasfase (Variables|Default|GetGalinhasFase))
  ;[0.15 0.15 0.15 0.5] Função responsável por reiniciar as váriáveis do jogo
  (Variables|Default|SetGalinhasSalvas_P1 0)
  (Variables|Default|SetGalinhasSalvas_P2 0)
  (Variables|Default|SetGalinhasAtropeladas_P1 0)
  (Variables|Default|SetGalinhasAtropeladas_P2 0)
  (Variables|Default|SetCountGalinhasAtropeladas 0)
  (if (Variables|Default|GetTimeTrial)
    (Variables|Default|SetTimer (Variables|Default|GetTempoFase))
    (else
      (Variables|Default|SetTimer 0.0)))
  ;;[0.15 0.15 0.15 0.5] Se forem 2 jogadores, marca que ambas as galinhas serão carregadas (ProxGalinha = 0) e ambos os ônibus são preenchidos. Para 1 jogador apenas a galinha do P1 é carregadas (ProxGalinha = 1) e o ônibus 2 recebe -1 (indicando que esta fora do jogo)
  (if (Variables|Default|Get2Players)
    (Variables|Default|SetProxGalinha 0)
    (Variables|Default|SetGalinhasOnibus_P2 _galinhasfase)
    (else
      (Variables|Default|SetProxGalinha 1)
      (Variables|Default|SetGalinhasOnibus_P2 -1)))
  (Variables|Default|SetGalinhasOnibus_P1 _galinhasfase)
  (Variables|Default|SetLevelGo true))

(fn UpdateHUDGalinhasAtropeladas
  ;[0.15 0.15 0.15 0.5] Atualiza o número de Galinhas Atropeladas no HUD
  (Default|UpdateGalinhasAtropeladas (Variables|Default|GetHUD_Ref) (Variables|Default|GetGalinhasAtropeladas_P1) (Variables|Default|GetGalinhasAtropeladas_P2)))

(fn UpdateHUDGalinhasSalvas
  ;[0.15 0.15 0.15 0.5] Atualiza o número de Galinhas Salvas no HUD
  (Default|UpdateGalinhasSalvas (Variables|Default|GetHUD_Ref) (Variables|Default|GetGalinhasSalvas_P1) (Variables|Default|GetGalinhasSalvas_P2)))

(fn UpdateHUDTempo
  ;[0.15 0.15 0.15 0.5] Atualiza o Tempo de jogo no HUD
  (Default|UpdateTempo (Variables|Default|GetHUD_Ref) (Variables|Default|GetTimer)))

(fn UpdateHUDGalinhasOnibus
  ;[0.15 0.15 0.15 0.5] Atualiza o número de Galinhas no ônibus no HUD
  (Default|UpdateGalinhasOnibus (Variables|Default|GetHUD_Ref) (Variables|Default|GetGalinhasOnibus_P1) (Variables|Default|GetGalinhasOnibus_P2)))

(fn SetControleTeclado
  (bind _returnvalue (Game|GetPlayerController 0))
  ;[0.15 0.15 0.15 0.5] Devolve o controle do jogo ao teclado
  (Variables|/Script/Engine.PlayerController|SetbShowMouseCursor _returnvalue false)
  (Input|SetInputModeGameOnly _returnvalue false))

(fn SetControleMouse
  (bind _returnvalue (Game|GetPlayerController 0))
  ;[0.15 0.15 0.15 0.5] Devolve o controle do jogo ao mouse
  (Variables|/Script/Engine.PlayerController|SetbShowMouseCursor _returnvalue true)
  (Input|SetInputModeUIOnly _returnvalue 0 "DoNotLock" false))

(fn ResetSpawns
  ;[0.15 0.15 0.15 0.5] Verifica se já existe um VeiculoSpawn no jogo (destroi e carrega um novo)
  (Utilities|IsValid (Variables|Default|GetVeiculoSpawn_Ref)
    (:Is%20Valid
      (Actor|DestroyActor (Variables|Default|GetVeiculoSpawn_Ref)))
    (:Is%20Not%20Valid
      _))
  (bind _returnvalue (Game|SpawnActorfromClass "/Game/BP_VeiculoSpawn.BP_VeiculoSpawn_C" (Math|Transform|MakeTransform "-200.000000,1500.000000,0.000000" "0, 0, 0" "1.000000,1.000000,1.000000") "Undefined" "MultiplyWithRoot" 0 0))
  (Variables|Default|SetVeiculoSpawn_Ref _returnvalue)
  ;[0.15 0.15 0.15 0.5] Faz o mesmo para o PowerUp Spawn
  (Utilities|IsValid (Variables|Default|GetPowerUpSpawn_Ref)
    (:Is%20Valid
      (Actor|DestroyActor (Variables|Default|GetPowerUpSpawn_Ref)))
    (:Is%20Not%20Valid
      _))
  (bind _returnvalue_2 (Game|SpawnActorfromClass "/Game/BP_PowerUpSpawn.BP_PowerUpSpawn_C" (Math|Transform|MakeTransform "-200.000000,1500.000000,0.000000" "0, 0, 0" "1.000000,1.000000,1.000000") "Undefined" "MultiplyWithRoot" 0 0))
  (Variables|Default|SetPowerUpSpawn_Ref _returnvalue_2))

(fn RemoveHud
  (bind _hud_ref (Variables|Default|GetHUD_Ref))
  ;[0.15 0.15 0.15 0.5] Verifica se o HUD existe e então remove o mesmo
  (Utilities|IsValid _hud_ref
    (:Is%20Valid
      (Widget|RemovefromParent _hud_ref))))

(fn CarregaHUD
  ;[0.15 0.15 0.15 0.5] Carrega o HUD do jogo na tela
  (bind _returnvalue (UserInterface|CreateWidget "/Game/_Widgets/WBP_Hud.WBP_Hud_C"))
  (bind _output_get (Variables|Default|SetHUD_Ref _returnvalue))
  (UserInterface|Viewport|AddtoViewport _output_get 0))

(fn ResetElementos
  (params (ElementoClass :type Actor%20Class%20Reference))
  ;[0.15 0.15 0.15 0.5] Verifica se existem na fase elementos da classe passada por referencia e então remove os mesmos
  (bind _outactors (Actor|GetAllActorsOfClass ElementoClass))
  (for _array_element _outactors
    (Actor|DestroyActor _array_element)))

(fn VerificaFimFase
  ;[0.15 0.15 0.15 0.5] Função que verifica se ambos os ônibus estão vazios, significando o final da fase.
  (if (< (Variables|Default|GetGalinhasOnibus_P1) 0)
    (if (< (Variables|Default|GetGalinhasOnibus_P2) 0)
      (CallFunction|FimFase))))

(fn AtualizaOnibus
  (params (Onibus_P1? :type Boolean))
  ;[0.15 0.15 0.15 0.5] Função que atualiza a quantidade de galinhas dentro do Ônibus
  (if Onibus_P1?
    (Variables|Default|SetGalinhasOnibus_P1 (- (Variables|Default|GetGalinhasOnibus_P1) 1))
    (else
      (Variables|Default|SetGalinhasOnibus_P2 (- (Variables|Default|GetGalinhasOnibus_P2) 1)))))

(fn CarregaGalinha
  (params (Onibus_P1? :type Boolean))
  ;[0.15 0.15 0.15 0.5] Carrega o Ator Galinha de acordo com o Player
  (if Onibus_P1?
    (bind _outactors (Actor|GetAllActorsOfClass "/Game/BP_Onibus_P1.BP_Onibus_P1_C"))
    (bind _returnvalue (Game|SpawnActorfromClass "/Game/BP_Galinha_P1.BP_Galinha_P1_C" (Math|Transform|MakeTransform (Transformation|GetWorldLocation (Variables|/Game/BP_Onibus_P1.BP_Onibus_P1_C|GetSpawnArrow (Utilities|Array|Get(acopy) _outactors))) "0, 0, 0" "1.000000,1.000000,1.000000") "Undefined" "MultiplyWithRoot" 0 0))
    (Pawn|Possess (Game|GetPlayerController 0) _returnvalue)
    (else
      (bind _outactors_2 (Actor|GetAllActorsOfClass "/Game/BP_Onibus_P2.BP_Onibus_P2_C"))
      (bind _returnvalue_2 (Game|SpawnActorfromClass "/Game/BP_Galinha_P2.BP_Galinha_P2_C" (Math|Transform|MakeTransform (Transformation|GetWorldLocation (Variables|/Game/BP_Onibus_P2.BP_Onibus_P2_C|GetSpawnArrow (Utilities|Array|Get(acopy) _outactors_2))) "0, 0, 0" "1.000000,1.000000,1.000000") "Undefined" "MultiplyWithRoot" 0 0))
      (Pawn|Possess (Game|GetPlayerController 1) _returnvalue_2))))

(fn CarregaOnibusP2
  ;[0.15 0.15 0.15 0.5] Deixa o ônibus referente ao Player 2 visível ou não dependendo da quantidade de jogadores
  (bind _outactors (Actor|GetAllActorsOfClass "/Game/BP_Onibus_P2.BP_Onibus_P2_C"))
  (if (Variables|Default|Get2Players)
    (Variables|Default|SetOnibus_P2_Z 7e+01)
    (else
      (Variables|Default|SetOnibus_P2_Z -2e+02)))
  (Transformation|SetWorldLocation (Variables|/Game/BP_Onibus_P2.BP_Onibus_P2_C|GetDefaultSceneRoot (Utilities|Array|Get(acopy) _outactors)) (Math|Vector|MakeVector (.x (Transformation|GetWorldLocation (Variables|/Game/BP_Onibus_P2.BP_Onibus_P2_C|GetDefaultSceneRoot (Utilities|Array|Get(acopy) _outactors)))) (.y (Transformation|GetWorldLocation (Variables|/Game/BP_Onibus_P2.BP_Onibus_P2_C|GetDefaultSceneRoot (Utilities|Array|Get(acopy) _outactors)))) (Variables|Default|GetOnibus_P2_Z)) false false))

(fn CarregaLapides
  (bind _countgalinhasatropeladas (Variables|Default|GetCountGalinhasAtropeladas))
  ;[0.15 0.15 0.15 0.5] Função que carrega uma quantidade de lápides de acordo com o número de galinhas que foram atropeladas
  (if (< _countgalinhasatropeladas (+ (Variables|Default|GetGalinhasAtropeladas_P1) (Variables|Default|GetGalinhasAtropeladas_P2))) :!label _label
    (bind _result (Math|Integer|IncrementInt _countgalinhasatropeladas)
      (:%20%20
        (Game|SpawnActorfromClass "/Game/BP_Lapide.BP_Lapide_C" (Math|Transform|MakeTransform (Math|Vector|MakeVector 3.5e+03 (Math|Conversions|ToFloat(Integer) (+ (* _result 100) 1200)) 0.0) "0, 0, 0" "1.000000,1.000000,1.000000") "Undefined" "MultiplyWithRoot" 0 0)
        (goto _label)))))

(fn PowerUpEfeitoVelocidade
  (params (GalinhaRef :type BP%20Galinha%20Object%20Reference))
  ;[0.15 0.15 0.15 0.5] Função que aumenta a velocidade da Galinha ao pegar o PowerUp de velocidade. Somente um PowerUp do tipo por Galinha
  (if (not (Variables|/Game/BP_Galinha.BP_Galinha_C|GetPowerUp_Velocidade? GalinhaRef))
    (Variables|/Game/BP_Galinha.BP_Galinha_C|SetSpeed GalinhaRef (* (Variables|/Game/BP_Galinha.BP_Galinha_C|GetSpeed GalinhaRef) (Variables|Default|GetPowerUp_Velocidade)))
    (Variables|/Game/BP_Galinha.BP_Galinha_C|SetPowerUp_Velocidade? GalinhaRef true)))

(fn PuloGalinha
  (params (GalinhaRef :type BP%20Galinha%20Object%20Reference))
  (bind _returnvalue (Transformation|GetActorLocation GalinhaRef))
  ;[0.15 0.15 0.15 0.5] Função que faz a Galinha Pular sobre o veículo em caso de resistência ao atropelamento. Pula pra cima e para frente.
  (Transformation|SetActorLocation GalinhaRef (Math|Vector|MakeVector (+ (.x _returnvalue) 1e+02) (.y _returnvalue) 5e+02) false false))

(fn PowerUpEfeitoResistencia
  (params (GalinhaRef :type BP%20Galinha%20Object%20Reference))
  ;[0.15 0.15 0.15 0.5] Função que aumenta a Vida (Resistência) da Galinha ao pegar o PowerUp de Resistência. Somente um PowerUp do tipo por Galinha
  (if (not (Variables|/Game/BP_Galinha.BP_Galinha_C|GetPowerUp_Resistencia? GalinhaRef))
    (Variables|/Game/BP_Galinha.BP_Galinha_C|SetResistencia GalinhaRef (Variables|Default|GetPowerUp_Resistencia))
    (Variables|/Game/BP_Galinha.BP_Galinha_C|SetPowerUp_Resistencia? GalinhaRef true)))