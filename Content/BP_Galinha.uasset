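; Player-controlled chicken that moves within screen bounds and shows a resistance power-up effect.
; BeginPlay caches the four screen limits from BP_GameMode; Tick applies swept movement from MovimentUp and MovimentRight, which are set outside these graphs.
; Chained edge checks block the whole move when heading past any limit.
; Unblocked ticks also toggle the particle from Resistencia, clearing the pickup flag when it is not above one.
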(event EventTick
  (params (DeltaSeconds :type Float%20%28single-precision%29))
  ;[0.15 0.15 0.15 0.5] Realiza a movimentação do personagem de acordo com o input do teclado e se houver espaço em tela para o movimento
  (bind _onscreen (CallFunction|CheckScreenLimits))
  (if _onscreen
    (Transformation|AddActorLocalOffset (Math|Vector|MakeVector (* DeltaSeconds (Variables|Default|GetMovimentUp)) (* DeltaSeconds (Variables|Default|GetMovimentRight)) 0.0) true false)
    (CallFunction|EfeitoPowerUpResistencia)))

(event EventBeginPlay
  ;[0.15 0.15 0.15 0.5] Busca as informações de limite de tela para travar a movimentação das galinhas
  (bind _asbp_game_mode (Utilities|Casting|CastToBP_GameMode (Game|GetGameMode)))
  (Variables|Default|SetLeftScreenLimit (Variables|/Game/BP_GameMode.BP_GameMode_C|GetLeftScreenLimit _asbp_game_mode))
  (Variables|Default|SetRightScreenLimit (Variables|/Game/BP_GameMode.BP_GameMode_C|GetRightScreenLimit _asbp_game_mode))
  (Variables|Default|SetDownScreenLimit (Variables|/Game/BP_GameMode.BP_GameMode_C|GetDownScreenLimit _asbp_game_mode))
  (Variables|Default|SetUpScreenLimit (Variables|/Game/BP_GameMode.BP_GameMode_C|GetUpScreenLimit _asbp_game_mode)))

(fn ConstructionScript)

(fn CheckLeftScreenLimit
  ;[0.15 0.15 0.15 0.5] Função que verifica se o jogador chegou ao limite ESQUERDO da tela e se ainda esta se movendo para esse lado (retorna falso travando o movimento). Caso ainda esteja dentro do limite ou se movendo no outro sentido, retorna verdadeiro.
  ;;[0.15 0.15 0.15 0.5] Verifica se o jogador passou o limite da tela
  (if (< (.y (Transformation|GetActorLocation)) (Variables|Default|GetLeftScreenLimit))
    ;;[0.15 0.15 0.15 0.5] Verifica se o jogador esta se movendo para o lado do limite (movimento negativo)
    (if (< (Variables|Default|GetMovimentRight) 0.0)
      (return false)
      (else
        _)))
  (return true))

(fn CheckRightScreenLimit
  ;[0.15 0.15 0.15 0.5] Função que verifica se o jogador chegou ao limite DIREITO da tela e se ainda esta se movendo para esse lado (retorna falso travando o movimento). Caso ainda esteja dentro do limite ou se movendo no outro sentido, retorna verdadeiro.
  ;;[0.15 0.15 0.15 0.5] Verifica se o jogador passou o limite da tela
  (if (> (.y (Transformation|GetActorLocation)) (Variables|Default|GetRightScreenLimit))
    ;;[0.15 0.15 0.15 0.5] Verifica se o jogador esta se movendo para o lado do limite (movimento positivo)
    (if (> (Variables|Default|GetMovimentRight) 0.0)
      (return false)
      (else
        _)))
  (return true))

(fn CheckDownScreenLimit
  ;[0.15 0.15 0.15 0.5] Função que verifica se o jogador chegou ao limite INFERIOR da tela e se ainda esta se movendo para esse lado (retorna falso travando o movimento). Caso ainda esteja dentro do limite ou se movendo no outro sentido, retorna verdadeiro.
  ;;[0.15 0.15 0.15 0.5] Verifica se o jogador passou o limite da tela
  (if (< (.x (Transformation|GetActorLocation)) (Variables|Default|GetDownScreenLimit))
    ;;[0.15 0.15 0.15 0.5] Verifica se o jogador esta se movendo para o lado do limite (movimento negativo)
    (if (< (Variables|Default|GetMovimentUp) 0.0)
      (return false)
      (else
        _)))
  (return true))

(fn CheckUpScreenLimit
  ;[0.15 0.15 0.15 0.5] Função que verifica se o jogador chegou ao limite SUPERIOR da tela e se ainda esta se movendo para esse lado (retorna falso travando o movimento). Caso ainda esteja dentro do limite ou se movendo no outro sentido, retorna verdadeiro.
  ;;[0.15 0.15 0.15 0.5] Verifica se o jogador passou o limite da tela
  (if (> (.x (Transformation|GetActorLocation)) (Variables|Default|GetUpScreenLimit))
    ;;[0.15 0.15 0.15 0.5] Verifica se o jogador esta se movendo para o lado do limite (movimento positivo)
    (if (> (Variables|Default|GetMovimentUp) 0.0)
      (return false)
      (else
        _)))
  (return true))

(fn CheckScreenLimits
  ;[0.15 0.15 0.15 0.5] Função que faz a verificação se o jogador esta dentro dos limites de tela ou não, travando o movimento em alguma direção se necessário
  (bind _onscreen (CallFunction|CheckLeftScreenLimit))
  (if _onscreen
    (bind _onscreen_2 (CallFunction|CheckRightScreenLimit))
    (if _onscreen_2
      (bind _onscreen_3 (CallFunction|CheckDownScreenLimit))
      (if _onscreen_3
        (bind _onscreen_4 (CallFunction|CheckUpScreenLimit))
        (if _onscreen_4
          (return true)
          (else
            _)))))
  (return false))

(fn EfeitoPowerUpResistencia
  (bind _particle_resistenciaon (Variables|Default|GetParticle_ResistenciaOn))
  ;[0.15 0.15 0.15 0.5] Função responsável por ligar/ desligar a indicação visual da Resistência aumentada, além de resetar a variável da coleta
  (Utilities|IsValid self
    (:Is%20Valid
      (if (> (Variables|Default|GetResistencia) 1)
        (Rendering|SetVisibility _particle_resistenciaon true false)
        (else
          (Rendering|SetVisibility _particle_resistenciaon false false)
          (Variables|Default|SetPowerUp_Resistencia? false))))))