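; BP_Galinha_P2 is the Player 2 chicken, a child Blueprint that specializes its parent for the second player.
; On BeginPlay it calls the parent and sets the Player2 flag.
; The MoveUp_P2 and MoveRight_P2 keyboard axes, scaled by Speed, write MovimentUp and MovimentRight; this graph does not apply the movement itself.
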(event EventBeginPlay
  ;[0.15 0.15 0.15 0.5] Marca as galinhas do Player 2
  (|CallParentFunction)
  (Variables|Default|SetPlayer2? true))

(event Collision|EventActorBeginOverlap
  (params (OtherActor :type Actor%20Object%20Reference)))

(event EventTick
  (params (DeltaSeconds :type Float%20%28single-precision%29))
  (|CallParentFunction DeltaSeconds) ; This node is disabled and will not be called.\nDrag off pins to build functionality.
)

(event Input|AxisEvents|InputAxisMoveUp_P2
  (params (AxisValue :type Float%20%28single-precision%29))
  ;[0.15 0.15 0.15 0.5] Busca a infomração de movimentação via teclado
  (Variables|Default|SetMovimentUp (* AxisValue (Variables|Default|GetSpeed))))

(event Input|AxisEvents|InputAxisMoveRight_P2
  (params (AxisValue :type Float%20%28single-precision%29))
  ;[0.15 0.15 0.15 0.5] Busca a infomração de movimentação via teclado
  (Variables|Default|SetMovimentRight (* (Variables|Default|GetSpeed) AxisValue)))

(fn ConstructionScript
  (|CallParentFunction))