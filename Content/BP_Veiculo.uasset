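; BP_Veiculo is a vehicle that can run over the chicken, BP_Galinha, and removes itself after a fixed lifespan.
; Its Box overlap stores the chicken it hits and reports the run-over to BP_GameMode through GalinhaAtropelada.
; A repeat overlap with that stored chicken, as with a truck, calls PuloGalinha on the cached game mode for another jump instead.
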(event OnComponentBeginOverlap(Box)
  (params (OverlappedComponent :type Primitive%20Component%20Object%20Reference) (OtherActor :type Actor%20Object%20Reference) (OtherComp :type Primitive%20Component%20Object%20Reference) (OtherBodyIndex :type Integer) (bFromSweep :type Boolean) (SweepResult :type Hit%20Result%20Structure%20%28by%20ref%29))
  ;[0.15 0.15 0.15 0.5] Chama a função referente ao atropelamento da Galinha. Se bater duas vezes no mesmo veículo (caminhão) um novo pulo é feito
  (bind _asbp_galinha (Utilities|Casting|CastToBP_Galinha OtherActor))
  (if (== _asbp_galinha (Variables|Default|GetGalinhaAtropelada))
    (Default|PuloGalinha (stale _asbp_game_mode) (stale _output_get))
    (else
      (bind _output_get (Variables|Default|SetGalinhaAtropelada _asbp_galinha))
      (bind _asbp_game_mode (Utilities|Casting|CastToBP_GameMode (Game|GetGameMode)))
      (Default|GalinhaAtropelada _asbp_game_mode _output_get))))

(event EventBeginPlay
  ;[0.15 0.15 0.15 0.5] Determina o tempo de vida do veículo
  (Actor|SetLifeSpan 25.0))

(fn ConstructionScript)