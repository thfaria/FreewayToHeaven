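; BP_VeiculoSpawn spawns vehicles on the road lanes at an interval set by the game mode's Trafigo (traffic) value.
; A looping timer started on BeginPlay calls SpawnVeiculo, which spawns the chosen ArrVeiculosSpawn entry's vehicle class with its position and direction.
; VerificaDisponibilidadePista picks a random lane, steps past recently used ones with wraparound, and rotates ArrPistasUtilizadas as a FIFO history to avoid quick repeats.
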(event EventBeginPlay
  ;[0.15 0.15 0.15 0.5] Dispara o Spawn dos veículos de acorod com o Tráfigo do Game Mode
  (bind _asbp_game_mode (Utilities|Casting|CastToBP_GameMode (Game|GetGameMode)))
  (Utilities|Time|SetTimerbyFunctionName 0 "SpawnVeiculo" (Variables|/Game/BP_GameMode.BP_GameMode_C|GetTrafigo _asbp_game_mode) true))

(fn ConstructionScript)

(fn SpawnVeiculo
  ;[0.15 0.15 0.15 0.5] Função que faz o veículo surgir na pista
  (bind _pistasorteada (CallFunction|VerificaDisponibilidadePista))
  (bind _output_get (LocalVariables|SetNewLocalVar (Utilities|Array|Get(acopy) (Variables|Default|GetArr_VeiculosSpawn) _pistasorteada)))
  (Game|SpawnActorfromClass (.tipo_veiculo _output_get) (Math|Transform|MakeTransform (Math|Vector|MakeVector (.posicao_x _output_get) (.posicao_y _output_get) 0.0) (.direcao _output_get) "1.000000,1.000000,1.000000") "Undefined" "MultiplyWithRoot" 0 0))

(fn VerificaDisponibilidadePista
  (bind _arr_pistasutilizadas (Variables|Default|GetArr_PistasUtilizadas))
  ;[0.15 0.15 0.15 0.5] Função que sorteia a pista a ser utilizada
  ;;[0.15 0.15 0.15 0.5] Verifica se a pista sorteada foi utilizada recentemente
  (bind _output_get (Variables|Default|SetPistaSorteada (Math|Random|RandomIntegerinRange 0 (- (Utilities|Array|Length (Variables|Default|GetArr_VeiculosSpawn)) 1))))
  (if (!= (Utilities|Array|FindItem (Variables|Default|GetArr_PistasUtilizadas) _output_get) -1) :!label _label
    ;;[0.15 0.15 0.15 0.5] Se tiver sido utilizada, soma 1 ao valor sorteado e verifica novamente
    (if (== (Variables|Default|GetPistaSorteada) (- (Utilities|Array|Length (Variables|Default|GetArr_VeiculosSpawn)) 1))
      (Variables|Default|SetPistaSorteada 0)
      (goto _label)
      (else
        (bind _result (Math|Integer|IncrementInt (Variables|Default|GetPistaSorteada))
          (:%20%20
            (Variables|Default|SetPistaSorteada _result)
            (goto _label)))))
    (else
      ;;[0.15 0.15 0.15 0.5] Se não encontrar, adiciona a pista a lista de pistas recentemente utilizadas e remove a última da lista
      (Utilities|Array|Add _arr_pistasutilizadas (Variables|Default|GetPistaSorteada))
      (Utilities|Array|RemoveIndex _arr_pistasutilizadas)
      ;;[0.15 0.15 0.15 0.5] Retorna a pista sorteada
      (return (Variables|Default|GetPistaSorteada)))))