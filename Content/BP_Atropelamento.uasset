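; BP_Atropelamento is a roadkill actor that gradually clears away as vehicles drive over it.
; BeginPlay puts a dynamic instance of MI_Atropelamento on its Sphere so its opacity can vary.
; Each BP_Veiculo overlap increments a pass counter and calls LimpaAtropelamento, which plays a clearing sound.
; That function keeps full opacity on the first pass, lowers it stepwise on later ones, and destroys the actor on the fourth.
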(event EventBeginPlay
  ;[0.15 0.15 0.15 0.5] Cria a instancia do material dinamico do atropelamento para poder variar sua transparencia
  (bind _returnvalue (Rendering|Material|CreateDynamicMaterialInstance "/Game/_Materials/MI_Atropelamento.MI_Atropelamento" "None" "None" :!class /Script/Engine.KismetMaterialLibrary))
  (bind _output_get (Variables|Default|SetMaterialDinamico _returnvalue))
  (Rendering|Material|SetMaterial (Variables|Default|GetSphere) 0 _output_get))

(event Collision|EventActorBeginOverlap
  (params (OtherActor :type Actor%20Object%20Reference))
  ;[0.15 0.15 0.15 0.5] Chama a função responsavel por limpar o atropelamento
  (Utilities|Casting|CastToBP_Veiculo OtherActor)
  (bind _result (Math|Integer|IncrementInt (Variables|Default|GetContPassagem))
    (:%20%20
      (Variables|Default|SetContPassagem _result)
      (CallFunction|LimpaAtropelamento))))

(fn ConstructionScript)

(fn LimpaAtropelamento
  ;[0.15 0.15 0.15 0.5] Função para a limpeza gradativa do atropelamento a medida que os carros vão passando por cima
  (Audio|PlaySound2D "/Game/Sounds/Clear.Clear" 1.0 1.0 1.0 0 0)
  (switch int (Variables|Default|GetContPassagem)
    (:1
      (Variables|Default|SetAtropelamentoVisibilidade 1.0)
      (Rendering|Material|SetScalarParameterValue (Variables|Default|GetMaterialDinamico) "Opacidade" (Variables|Default|GetAtropelamentoVisibilidade) :!class /Script/Engine.MaterialInstanceDynamic :!label _label)
      (Rendering|Material|SetMaterial (Variables|Default|GetSphere) 0 (Variables|Default|GetMaterialDinamico)))
    (:2
      (Variables|Default|SetAtropelamentoVisibilidade 0.75)
      (goto _label))
    (:3
      (Variables|Default|SetAtropelamentoVisibilidade 0.5)
      (goto _label))
    (:4
      (Actor|DestroyActor))))