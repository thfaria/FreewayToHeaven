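; BP_Alma is a soul actor that hovers in place briefly after spawning, then rises into the sky and is destroyed.
; On BeginPlay it stores its initial Z and plays the FlutuacaoAlma timeline, scaled by Amplitude, to bob vertically.
; After a short delay it stops that timeline and plays Ascender, which offsets Z from the same initial height and destroys the actor when finished.
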(event EventBeginPlay
  (bind _returnvalue (Transformation|GetActorLocation))
  (Utilities|FlowControl|Sequence
    (:then_0
      ;[0.15 0.15 0.15 0.5] Armazena a posição Z inicial da alma, aplica a flutuação e a amplitude
      (bind _output_get (Variables|Default|SetZInicial (.z _returnvalue)))
      (bind _flutuar (Timeline|FlutuacaoAlma Play)
        (:Update
          (Transformation|SetActorLocation (Math|Vector|MakeVector (.x _returnvalue) (.y _returnvalue) (+ (* _flutuar (Variables|Default|GetAmplitude)) _output_get)) false false))))
    (:then_1
      ;[0.15 0.15 0.15 0.5] Depois de alguns segundos a alma ascende aos céus e o ator é destruido
      (Utilities|FlowControl|Delay 2.5)
      (Utilities|FlowControl|Sequence
        (:then_0
          (Timeline|FlutuacaoAlma Stop))
        (:then_1
          (bind _ascender (Timeline|Ascender Play)
            (:Update
              (Transformation|SetActorLocation (Math|Vector|MakeVector (.x _returnvalue) (.y _returnvalue) (+ _output_get _ascender)) false false))
            (:Finished
              (Actor|DestroyActor))))))))

(fn ConstructionScript)